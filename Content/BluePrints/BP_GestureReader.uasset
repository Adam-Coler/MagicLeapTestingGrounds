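; BP_GestureReader detects Magic Leap static hand gestures and registers itself with BP_GameMode as the gesture reader.
; On play it configures tracked gestures and confidence thresholds, both adjustable at runtime.
; Gesture key presses fire OnGestureDetected, which updates per-hand state for queries and fires GestureUpdated.
; Right-hand key events also report LeftHand, so these inputs only update the left-hand gesture.
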(event Custom|SetCurrentGestures
  (params (Gesture :type EHandTrackingGesture%20Enum :default "Finger") (Hand :type E_HandType%20Enum :default "NewEnumerator0"))
  ;[1 0.1853 0] Save current gestures for each hand
  (Gestures|UpdateCurrentGestures Gesture Hand))

(event EventBeginPlay
  ;[0.165 1 0.1379] Initialize
  (Utilities|FlowControl|Sequence
    (:then_0
      (Input|EnableInput (Game|GetPlayerController 0)))
    (:then_1
      (Class|MagicLeapHandTrackingFunctionLibrary|SetConfiguration (Variables|Gestures|GetActiveStaticGestures) "NoFilter" "NoFilter" "NoFilter" true)
      (for _array_element (Variables|Gestures|GetActiveStaticGestures)
        (Class|MagicLeapHandTrackingFunctionLibrary|SetStaticGestureConfidenceThreshold _array_element (Variables|Gestures|GetGestureConfidenceThreshold))))
    (:then_2
      (EventDispatchers|BindEventtoOnGestureDetected (delegate Custom|SetCurrentGestures)))
    (:then_3
      (bind _asbp_game_mode (Utilities|Casting|CastToBP_GameMode (Game|GetGameMode)))
      (Variables|/Game/Maps/BP_GameMode.BP_GameMode_C|SetGestureReader _asbp_game_mode self))))

(event EventEndPlay
  (params (EndPlayReason :type EEndPlayReason%20Enum :default "Destroyed"))
  ;[1 0.165 0.1379] Finalize
  (Class|MagicLeapHandTrackingFunctionLibrary|SetConfiguration (Utilities|Array|MakeArray "NoHand") "NoFilter" "NoFilter" "NoFilter" true))

(event Input|KeyboardEvents|MagicLeapLeftThumb
  (params (Key :type Key%20Structure))
  ;[0.1451 0.003922 0.003922] Left Hand - Gesture Events
  (:Pressed
    (Default|CallOnGestureDetected "Thumb" "NewEnumerator0")))

(event Input|KeyboardEvents|MagicLeapLeftC
  (params (Key :type Key%20Structure))
  ;[0.1451 0.003922 0.003922] Left Hand - Gesture Events
  (:Pressed
    (Default|CallOnGestureDetected "C" "NewEnumerator0")))

(event Input|KeyboardEvents|MagicLeapRightFinger
  (params (Key :type Key%20Structure))
  ;[0.1441 0.003677 0.003677] Right Hand - Gesture Events
  (:Pressed
    (Default|CallOnGestureDetected "Finger" "NewEnumerator0")))

(event Input|KeyboardEvents|MagicLeapRightFist
  (params (Key :type Key%20Structure))
  ;[0.1441 0.003677 0.003677] Right Hand - Gesture Events
  (:Pressed
    (Default|CallOnGestureDetected "Fist" "NewEnumerator0")))

(event Input|KeyboardEvents|MagicLeapRightPinch
  (params (Key :type Key%20Structure))
  ;[0.1441 0.003677 0.003677] Right Hand - Gesture Events
  (:Pressed
    (Default|CallOnGestureDetected "Pinch" "NewEnumerator0")))

(event Input|KeyboardEvents|MagicLeapRightThumb
  (params (Key :type Key%20Structure))
  ;[0.1441 0.003677 0.003677] Right Hand - Gesture Events
  (:Pressed
    (Default|CallOnGestureDetected "Thumb" "NewEnumerator0")))

(event Input|KeyboardEvents|MagicLeapLeftFinger
  (params (Key :type Key%20Structure))
  ;[0.1451 0.003922 0.003922] Left Hand - Gesture Events
  (:Pressed
    (Default|CallOnGestureDetected "Finger" "NewEnumerator0")))

(event Input|KeyboardEvents|MagicLeapRightL
  (params (Key :type Key%20Structure))
  ;[0.1441 0.003677 0.003677] Right Hand - Gesture Events
  (:Pressed
    (Default|CallOnGestureDetected "L" "NewEnumerator0")))

(event Input|KeyboardEvents|MagicLeapRightOpenHandBack
  (params (Key :type Key%20Structure))
  ;[0.1441 0.003677 0.003677] Right Hand - Gesture Events
  (:Pressed
    (Default|CallOnGestureDetected "OpenHandBack" "NewEnumerator0")))

(event Input|KeyboardEvents|MagicLeapRightOk
  (params (Key :type Key%20Structure))
  ;[0.1441 0.003677 0.003677] Right Hand - Gesture Events
  (:Pressed
    (Default|CallOnGestureDetected "Ok" "NewEnumerator0")))

(event Input|KeyboardEvents|MagicLeapRightC
  (params (Key :type Key%20Structure))
  ;[0.1441 0.003677 0.003677] Right Hand - Gesture Events
  (:Pressed
    (Default|CallOnGestureDetected "C" "NewEnumerator0")))

(event Input|KeyboardEvents|MagicLeapRightNoHand
  (params (Key :type Key%20Structure))
  ;[0.1441 0.003677 0.003677] Right Hand - Gesture Events
  (:Pressed
    (Default|CallOnGestureDetected "NoHand" "NewEnumerator0")))

(event Input|KeyboardEvents|MagicLeapLeftFist
  (params (Key :type Key%20Structure))
  ;[0.1451 0.003922 0.003922] Left Hand - Gesture Events
  (:Pressed
    (Default|CallOnGestureDetected "Fist" "NewEnumerator0")))

(event Input|KeyboardEvents|MagicLeapLeftL
  (params (Key :type Key%20Structure))
  ;[0.1451 0.003922 0.003922] Left Hand - Gesture Events
  (:Pressed
    (Default|CallOnGestureDetected "L" "NewEnumerator0")))

(event Input|KeyboardEvents|MagicLeapLeftNoHand
  (params (Key :type Key%20Structure))
  ;[0.1451 0.003922 0.003922] Left Hand - Gesture Events
  (:Pressed
    (Default|CallOnGestureDetected "NoHand" "NewEnumerator0")))

(event Input|KeyboardEvents|MagicLeapLeftOk
  (params (Key :type Key%20Structure))
  ;[0.1451 0.003922 0.003922] Left Hand - Gesture Events
  (:Pressed
    (Default|CallOnGestureDetected "Ok" "NewEnumerator0")))

(event Input|KeyboardEvents|MagicLeapLeftOpenHandBack
  (params (Key :type Key%20Structure))
  ;[0.1451 0.003922 0.003922] Left Hand - Gesture Events
  (:Pressed
    (Default|CallOnGestureDetected "OpenHandBack" "NewEnumerator0")))

(event Input|KeyboardEvents|MagicLeapLeftPinch
  (params (Key :type Key%20Structure))
  ;[0.1451 0.003922 0.003922] Left Hand - Gesture Events
  (:Pressed
    (Default|CallOnGestureDetected "Pinch" "NewEnumerator0")))

(fn ConstructionScript)

(fn IsGestureActive
  (params (Gesture :type EHandTrackingGesture%20Enum :default "Finger") (Hand :type E_HandType%20Enum :default "NewEnumerator0"))
  (bind _currentleftgesture (Variables|Gestures|GetCurrentLeftGesture))
  (bind _currentrightgesture (Variables|Gestures|GetCurrentRightGesture))
  (bind _returnvalue (Utilities|Enum|Equal(Enum) Gesture _currentrightgesture))
  (bind _returnvalue_2 (Utilities|Enum|Equal(Enum) _currentleftgesture Gesture))
  (switch Utilities|FlowControl|Switch|SwitchonE_HandType Hand
    (:NewEnumerator0
      ;[1 1 1] Matching hand and gesture
      (return (Utilities|Enum|Equal(Enum) (Variables|Gestures|GetCurrentLeftGesture) Gesture) 0))
    (:NewEnumerator1
      (return (Utilities|Enum|Equal(Enum) Gesture (Variables|Gestures|GetCurrentRightGesture)) 0))
    (:NewEnumerator2
      ;[1 1 1] Check if any hand matches gesture and report that info back to caller
      (if (and _returnvalue_2 _returnvalue)
        (return true 0)
        (elif _returnvalue_2
          (return true 0)
          (else
            (return _returnvalue 0)))))))

(fn GetCurrentGesture
  (params (Hand :type E_HandType%20Enum :default "NewEnumerator0"))
  (bind _currentleftgesture (Variables|Gestures|GetCurrentLeftGesture))
  (switch Utilities|FlowControl|Switch|SwitchonE_HandType Hand
    (:NewEnumerator0
      (return (Variables|Gestures|GetCurrentLeftGesture)))
    (:NewEnumerator1
      (return (Variables|Gestures|GetCurrentRightGesture)))
    (:NewEnumerator2
      ;[1 1 1] When requesting both hands, try to give left gesture if valid, otherwise give whatever right is
      (return (select (Utilities|Enum|Equal(Enum) _currentleftgesture "NoHand") (Variables|Gestures|GetCurrentRightGesture) _currentleftgesture)))))

(fn UpdateCurrentGestures
  (params (Gesture :type EHandTrackingGesture%20Enum :default "Finger") (Hand :type E_HandType%20Enum :default "NewEnumerator0"))
  (Utilities|FlowControl|Sequence
    (:then_0
      (if (Utilities|Enum|Equal(Enum) Hand "NewEnumerator0")
        (Variables|Gestures|SetCurrentLeftGesture Gesture)
        (else
          (Variables|Gestures|SetCurrentRightGesture Gesture))))
    (:then_1
      (Default|CallGestureUpdated))))

(fn SetGestureTrackingStatus
  (params (Gesture :type EHandTrackingGesture%20Enum :default "Finger") (Tracked :type Boolean))
  (bind _activestaticgestures (Variables|Gestures|GetActiveStaticGestures))
  (bind _activestaticgestures_2 (Variables|Gestures|GetActiveStaticGestures))
  (bind _returnvalue (Utilities|Array|ContainsItem _activestaticgestures Gesture))
  (if Tracked
    ;[1 1 1] Only take action when state has changed
    (if (not _returnvalue)
      ;[1 1 1] Update active gestures
      (Utilities|FlowControl|Sequence
        (:then_0
          (Utilities|Array|Add _activestaticgestures_2 Gesture))
        (:then_1
          (Class|MagicLeapHandTrackingFunctionLibrary|SetConfiguration (Variables|Gestures|GetActiveStaticGestures) "NoFilter" "NoFilter" "NoFilter" true :!label _label))))
    (elif _returnvalue
      (Utilities|FlowControl|Sequence
        (:then_0
          (Utilities|Array|RemoveItem _activestaticgestures_2 Gesture))
        (:then_1
          (goto _label))))))

(fn GetActiveGestures
  (return (Variables|Gestures|GetActiveStaticGestures)))

(fn SetGestureConfidenceThreshold
  (params (NewConfidence :type Float%20%28single-precision%29))
  (Utilities|FlowControl|Sequence
    (:then_0
      (bind _output_get (Variables|Gestures|SetGestureConfidenceThreshold NewConfidence)))
    (:then_1
      (for _array_element (Variables|Gestures|GetActiveStaticGestures)
        (Class|MagicLeapHandTrackingFunctionLibrary|SetStaticGestureConfidenceThreshold _array_element _output_get)))))