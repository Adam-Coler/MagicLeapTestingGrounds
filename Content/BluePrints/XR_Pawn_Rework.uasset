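; Magic Leap XR pawn that drives controller and hand-gesture interaction with physics objects, plus level-specific menus.
; Controller traces feed the beam, hover highlighting, cube spawning and PhysicsHandle grabbing, with input to rotate, scale and extend held objects.
; Left-hand GestureReader poses grab or drop objects found by a capsule trace.
; Menu widgets soft-lock to camera view by interpolation, while a double-click macro overloads the home and shoulder buttons.
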(event OnTouchpadGestureStart(TouchpadGestures)
  (params (GestureData :type Magic%20Leap%20Touchpad%20Gesture%20Structure%20%28by%20ref%29)))

(event OnTouchpadGestureEnd(TouchpadGestures)
  (params (GestureData :type Magic%20Leap%20Touchpad%20Gesture%20Structure%20%28by%20ref%29)))

(event Custom|WidgetSoftlock
  (params (DeltaSeconds :type Float%20%28single-precision%29))
  (bind _returnvalue (Game|GetPlayerCameraManager 0))
  (bind _widget (Variables|Default|GetWidget))
  (bind _widget_gestures (Variables|Default|GetWidget_Gestures))
  (bind _returnvalue_2 (Transformation|GetWorldLocation _widget))
  (bind _returnvalue_3 (Camera|GetCameraLocation _returnvalue))
  (bind _returnvalue_4 (Math|Rotator|FindLookatRotation _returnvalue_2 _returnvalue_3))
  ;[0 0 0] Widget Softlock. Interps between current position and positon from previous tick
  (bind _output_get (Variables|Default|SetLocationTarget (+ _returnvalue_3 (* (Transformation|GetActorForwardVector _returnvalue) (Variables|Default|GetWidgetDistance)))))
  (bind _output_get_2 (Variables|Default|SetLocationCurrent (Math|Vector|Lerp(Vector) (Variables|Default|GetLocationCurrent) _output_get (* DeltaSeconds (Variables|Default|GetWidgetInterpSpeed)))))
  (Transformation|SetWorldLocation _widget _output_get_2 false false)
  (Transformation|SetWorldRotation _widget _returnvalue_4 false false)
  (Transformation|SetWorldLocation _widget_gestures _output_get_2 false false)
  (Transformation|SetWorldRotation _widget_gestures _returnvalue_4 false false))

(event Custom|TickSetGrabLocation
  (bind _motioncontroller (Variables|Default|GetMotionController))
  (bind _physicshandle (Variables|Default|GetPhysicsHandle))
  ;[1 1 1] Set Grabbed Object Location
  (if (Variables|Grabber|GetIsGestureGrab)
    (Physics|Components|PhysicsHandle|SetTargetLocation _physicshandle (Variables|GestureInteraction|GetLeftHandPosition))
    (else
      (Physics|Components|PhysicsHandle|SetTargetLocation _physicshandle (+ (Transformation|GetWorldLocation _motioncontroller) (* (Math|Vector|GetForwardVector _motioncontroller) (Variables|Grabber|GetGrabberDistance)))))))

(event Custom|SetWidgetScale
  (bind _widget (Variables|Default|GetWidget))
  ;[1 1 1] Setup Hide show widget
  (Utilities|FlowControl|Sequence
    (:then_0
      (if (Variables|Default|GetEnableWidget)
        (Variables|Default|SetEnableWidget false)
        (Transformation|SetWorldScale3D _widget "0, 0, 0")
        (else
          (Variables|Default|SetEnableWidget true)
          (Transformation|SetWorldScale3D _widget (Math|Conversions|ToVector(Float) (Variables|Default|GetWidgetScale))))))))

(event Custom|SetGrabberObjectRotation
  (bind _motioncontroller (Variables|Default|GetMotionController))
  (bind _returnvalue (Transformation|GetRelativeTransform _motioncontroller))
  (bind _rotation (Math|Transform|BreakTransform _returnvalue))
  ;[1 1 1] Rotate grabbed object with controller
  (if (and (!= (Variables|Grabber|GetGrabbedObject) 0) (Variables|Grabber|GetObjectGrabbed))
    (Math|Float|CompareFloat (Math|Float|Absolute(Float) (.roll _rotation)) 3e+01
      (:>
        (Transformation|AddRelativeRotation (Variables|Grabber|GetGrabbedObject) (Math|Rotator|MakeRotator 0.0 0.0 (* (.roll _rotation) 0.1)) false false)))))

(event Custom|yurp
  (params (bSuccess :type Boolean) (FilePath :type String))
  (Development|PrintText (Utilities|Text|ToText(String) (Utilities|String|Append "Donkey  " (Utilities|String|ToString(Boolean) bSuccess) " : " FilePath))))

(event Custom|PickUp
  ;[1 1 1] Pickup Object
  (bind (_hitcomponent _objecthit _location) (CallFunction|FLineTracefromController))
  (CallFunction|FGrabObject _hitcomponent _objecthit _location))

(event Custom|GestureUpdated
  ;[1 1 1] Begin Play
  (CallFunction|GesturePresentTest))

(event Custom|TestGestureCollision
  (Utilities|FlowControl|Sequence
    (:then_0
      (if (Variables|GestureInteraction|GetLeftHandPresent)
        (CallFunction|HandGestureCollision (Variables|GestureInteraction|GetLeftHandPosition))))))

(event Custom|HandGestureCollision
  (params (Position :type Vector))
  (bind (_hitcomponent _ishit _location) (CallFunction|FGestureCollision Position))
  (if _ishit
    (CallFunction|FObjectHovered _hitcomponent)
    (switch Utilities|FlowControl|Switch|SwitchonEHandTrackingGesture (Default|GetCurrentGesture (Variables|Default|GetGestureReader) "NewEnumerator0")
      (:Finger
        (CallFunction|FDropObject :!label _label)
        (Variables|Grabber|SetIsGestureGrab false))
      (:Fist
        (CallFunction|FGrabObject _hitcomponent _ishit _location :!label _label_2)
        (Variables|Grabber|SetIsGestureGrab true))
      (:Pinch
        (goto _label_2))
      (:Thumb
        (goto _label))
      (:L
        (goto _label))
      (:OpenHandBack
        (goto _label))
      (:Ok
        (goto _label_2))
      (:C
        (goto _label_2))
      (:NoPose
        (goto _label))
      (:NoHand
        (goto _label)))))

(event Custom|BtnPressIntro
  ;[0 0 0] Quit Game on Home Press Right
  (Game|OpenLevel(byName) "Meshing"))

(event Custom|GesturePresentTest
  (bind _gesturereader (Variables|Default|GetGestureReader))
  (bind _gesturereader_2 (Variables|Default|GetGestureReader))
  ;[1 1 1] Are Hands Present and fetch positions
  (Utilities|FlowControl|Sequence
    (:then_0
      (switch Utilities|FlowControl|Switch|SwitchonEHandTrackingGesture (Default|GetCurrentGesture _gesturereader_2 "NewEnumerator0")
        (:Finger
          (Variables|GestureInteraction|SetLeftHandPresent true :!label _label))
        (:Fist
          (goto _label))
        (:Pinch
          (goto _label))
        (:Thumb
          (goto _label))
        (:L
          (goto _label))
        (:OpenHandBack
          (goto _label))
        (:Ok
          (goto _label))
        (:C
          (goto _label))
        (:NoPose
          (Variables|GestureInteraction|SetLeftHandPresent false :!label _label_2))
        (:NoHand
          (goto _label_2)))
      (bind _lefthandcenter (Default|GetHandPosition _gesturereader "NewEnumerator0"))
      (Variables|GestureInteraction|SetLeftHandPosition _lefthandcenter))
    (:then_1
      (switch Utilities|FlowControl|Switch|SwitchonEHandTrackingGesture (Default|GetCurrentGesture _gesturereader_2 "NewEnumerator1")
        (:Finger
          (Variables|GestureInteraction|SetRightHandPresent true :!label _label_3))
        (:Fist
          (goto _label_3))
        (:Pinch
          (goto _label_3))
        (:Thumb
          (goto _label_3))
        (:L
          (goto _label_3))
        (:OpenHandBack
          (goto _label_3))
        (:Ok
          (goto _label_3))
        (:C
          (goto _label_3))
        (:NoPose
          (Variables|GestureInteraction|SetRightHandPresent false :!label _label_4))
        (:NoHand
          (goto _label_4)))
      (bind _righthandcenter (Default|GetHandPosition _gesturereader "NewEnumerator1"))
      (Variables|GestureInteraction|SetRightHandPosition _righthandcenter))))

(event Custom|Set%20Widget%20to%20Help
  ;[1 1 1] Set up menu btn selection
  (bind _returnvalue (CallFunction|FSetWidgetHelp)))

(event Custom|Drop
  ;[1 1 1] Drop Object
  (CallFunction|FDropObject))

(event Custom|Set%20Widget%20to%20Intro
  ;[1 1 1] Set up menu btn selection
  (bind _intro (CallFunction|FSetWidgetIntro)))

(event Custom|ObjectHovered
  ;[1 1 1] On controller hover change color
  (if (not (Math|Boolean|ORBoolean (Variables|Default|GetTriggerPressed) (Variables|Grabber|GetObjectGrabbed) (Variables|Default|GetEnableWidget)))
    (bind _hitcomponent (CallFunction|FLineTracefromController))
    (CallFunction|FObjectHovered _hitcomponent)))

(event Custom|Set%20Widget%20toMeshing
  ;[1 1 1] Set up menu btn selection
  (bind _meshing_menu (CallFunction|FSetWidgetMeshing)))

(event Custom|setWidget
  (bind _widget_gestures (Variables|Default|GetWidget_Gestures))
  ;[1 1 1] sET mAIN wIDGET TO MESH OR HELP
  (Utilities|FlowControl|Sequence
    (:then_0
      (if (Variables|Default|GetIsMainWidget)
        (Variables|Default|SetIsMainWidget false)
        (CallFunction|SetWidgettoHelp)
        (Transformation|SetWorldScale3D _widget_gestures "0, 0, 0")
        (else
          (Variables|Default|SetIsMainWidget true)
          (CallFunction|SetWidgettoMeshing)
          (Transformation|SetWorldScale3D _widget_gestures (Math|Conversions|ToVector(Float) (Variables|Default|GetWidgetScale))))))))

(event EventBeginPlay
  ;[1 1 1] Begin Play
  (bind _asbp_game_mode (Utilities|Casting|CastToBP_GameMode (Game|GetGameMode)))
  (bind _output_get (Variables|/Game/Maps/BP_GameMode.BP_GameMode_C|SetXR_Pawn _asbp_game_mode self))
  (Utilities|FlowControl|Sequence
    (:then_0
      (Pawn|Possess (Game|GetPlayerController 0) _output_get)
      (Utilities|IsValid (Variables|/Game/BluePrints/XR_Pawn.XR_Pawn_C|GetMotionController _output_get)
        (:Is%20Valid
          (Variables|/Script/HeadMountedDisplay.MotionControllerComponent|SetMotionSource (Variables|/Game/BluePrints/XR_Pawn.XR_Pawn_C|GetMotionController _output_get) "Right"))))
    (:then_1
      (bind _returnvalue (Game|GetCurrentLevelName true))
      (switch string _returnvalue
        (:Intro
          (CallFunction|SetWidgettoIntro))
        (:Meshing
          (Utilities|FlowControl|Sequence
            (:then_0
              (CallFunction|SetWidgettoMeshing)
              (Variables|Default|SetIsMainWidget true))
            (:then_1
              (CallFunction|FSetWidgetGestures))))))
    (:then_2
      (if (Variables|GestureInteraction|GetGestureInteractionEnabled)
        (bind _output_get_2 (Variables|Default|SetGestureReader (Variables|/Game/Maps/BP_GameMode.BP_GameMode_C|GetGestureReader _asbp_game_mode)))
        (EventDispatchers|BindEventtoGestureUpdated _output_get_2 (delegate Custom|GestureUpdated))))))

(event EventTick
  (params (DeltaSeconds :type Float%20%28single-precision%29))
  ;[1 0 1] Tick
  (CallFunction|FSoftLock (Variables|Default|GetWidget))
  (CallFunction|FSoftLock (Variables|Default|GetWidget_Gestures))
  (Utilities|FlowControl|Sequence
    (:then_0
      (if (Variables|Grabber|GetObjectGrabbed)
        (CallFunction|TickSetGrabLocation)))
    (:then_1
      (if (not (or (Variables|Default|GetTriggerPressed) (Variables|Default|GetEnableWidget)))
        (CallFunction|FDrawRayTraceControllertoCollision)))
    (:then_2
      (CallFunction|ObjectHovered))
    (:then_3
      (if (Variables|Grabber|GetObjectGrabbed)
        (CallFunction|SetGrabberObjectRotation)))
    (:then_4
      (if (and (Variables|GestureInteraction|GetGestureInteractionEnabled) (or (Variables|GestureInteraction|GetLeftHandPresent) (Variables|GestureInteraction|GetRightHandPresent)))
        (CallFunction|GesturePresentTest)
        (CallFunction|TestGestureCollision)))))

(event Input|KeyboardEvents|MotionControllerRightTrigger
  (params (Key :type Key%20Structure))
  ;[1 1 1] Grabber Input Binding
  (:Pressed
    (CallFunction|PickUp)
    (Variables|Grabber|SetIsGestureGrab false :!label _label))
  (:Released
    (CallFunction|Drop)
    (goto _label)))

(event Input|KeyboardEvents|MotionControllerRightThumbstick
  (params (Key :type Key%20Structure))
  ;[1 1 1] Set up menu btn selection
  (:Pressed
    (if (not (Variables|Default|GetIsMainWidget))
      (CallFunction|FSetWidgetMenuHoverSelection (stale Custom|Set%20Widget%20to%20Help _returnvalue))
      (Class|MagicLeapControllerFunctionLibrary|PlayHapticPattern "Right" "None" "Low"))))

(event Input|KeyboardEvents|MotionControllerRightThumbstick
  (params (Key :type Key%20Structure))
  ;[1 1 1] Set up menu btn selection
  (:Pressed
    (CallFunction|FSetWidgetMenuHoverSelection (stale Custom|Set%20Widget%20to%20Intro _intro))
    (Class|MagicLeapControllerFunctionLibrary|PlayHapticPattern "Right" "None" "Low")))

(event Input|KeyboardEvents|MotionControllerRightThumbstick
  (params (Key :type Key%20Structure))
  ;[1 1 1] Set up menu btn selection
  (:Pressed
    (if (Variables|Default|GetIsMainWidget)
      (CallFunction|FSetWidgetMenuHoverSelection (stale Custom|Set%20Widget%20toMeshing _meshing_menu))
      (Class|MagicLeapControllerFunctionLibrary|PlayHapticPattern "Right" "None" "Low"))))

(event Input|KeyboardEvents|MotionControllerRightTrigger
  (params (Key :type Key%20Structure))
  ;[1 1 1] Set up menu btn selection
  (:Pressed
    (if (Variables|Default|GetIsMainWidget)
      (CallFunction|FSetMenuHoverClickEvent (stale Custom|Set%20Widget%20toMeshing _meshing_menu))
      (Class|MagicLeapControllerFunctionLibrary|PlayHapticPattern "Right" "None" "Low"))))

(event Input|KeyboardEvents|MagicLeapRightHomeButton
  (params (Key :type Key%20Structure))
  ;[1 1 1] Haptics
  (:Pressed
    (Audio|PlaySound2D "/Game/Sounds/ui_confirm_short.ui_confirm_short" 1.0 1.0 0.0 0 0)
    (Class|MagicLeapControllerFunctionLibrary|PlayHapticPattern "Right" "ForceDown" "Low")))

(event Input|KeyboardEvents|MotionControllerRightShoulder
  (params (Key :type Key%20Structure))
  ;[1 1 1] Haptics
  (:Pressed
    (Audio|PlaySound2D "/Game/Sounds/ui_confirm_short.ui_confirm_short" 1.0 1.0 0.0 0 0)
    (Class|MagicLeapControllerFunctionLibrary|PlayHapticPattern "Right" "ForceDown" "Low")))

(event Input|KeyboardEvents|MotionControllerRightTrigger
  (params (Key :type Key%20Structure))
  ;[1 1 1] Set up menu btn selection
  (:Pressed
    (CallFunction|FSetMenuHoverClickEvent (stale Custom|Set%20Widget%20to%20Intro _intro))
    (Class|MagicLeapControllerFunctionLibrary|PlayHapticPattern "Right" "None" "Low")))

(event Input|KeyboardEvents|MotionControllerRightShoulder
  (params (Key :type Key%20Structure))
  ;[1 1 1] Spawn Object
  (:Pressed
    (Utilities|DetectDoubleClick
      (:Double%20Click
        (Class|CameraCaptureComponent|CaptureImagetoFileAsync (Variables|Default|GetCameraCapture) (delegate Custom|yurp)))
      (:Single%20Click
        (CallFunction|FSpawnObjectatCursor)))))

(event Input|KeyboardEvents|MotionControllerRightTrigger
  (params (Key :type Key%20Structure))
  ;[1 1 1] Draw Beam
  (:Pressed
    (Variables|Default|SetTriggerPressed true))
  (:Released
    (Variables|Default|SetTriggerPressed false)))

(event Input|KeyboardEvents|MotionControllerRightTrigger
  (params (Key :type Key%20Structure))
  ;[1 1 1] Set up menu btn selection
  (:Pressed
    (if (not (Variables|Default|GetIsMainWidget))
      (CallFunction|FSetMenuHoverClickEvent (stale Custom|Set%20Widget%20to%20Help _returnvalue))
      (Class|MagicLeapControllerFunctionLibrary|PlayHapticPattern "Right" "None" "Low"))))

(event Input|KeyboardEvents|MagicLeapRightHomeButton
  (params (Key :type Key%20Structure))
  ;[0 0 0] Quit Game on Home Press Right
  (:Pressed
    (Utilities|DetectDoubleClick
      (:Double%20Click
        (bind _returnvalue (Game|GetCurrentLevelName true))
        (if (Utilities|Enum|Equal(Enum) _returnvalue "Intro")
          (Game|OpenLevel(byName) "Meshing")
          (else
            (Game|QuitGame 0 "Quit" false))))
      (:Single%20Click
        (CallFunction|SetWidgetScale)
        (CallFunction|FShrinkBeam)))))

(event Input|KeyboardEvents|MotionControllerRightThumbstick
  (params (Key :type Key%20Structure))
  (bind _returnvalue (Class|Actor|GetInputAxisKeyValue))
  (bind _returnvalue_2 (Class|Actor|GetInputAxisKeyValue))
  (bind _returnvalue_3 (Class|Actor|GetInputAxisKeyValue))
  ;[1 1 1] Grabber Scale, Extend
  (:Pressed
    (if (Variables|Grabber|GetObjectGrabbed)
      (Utilities|FlowControl|Sequence
        (:then_0
          (Math|Float|CompareFloat (Math|Float|Absolute(Float) _returnvalue_3) 0.5
            (:>
              (Variables|Grabber|SetGrabberDistance (+ (* _returnvalue_3 (* _returnvalue_2 2e+02)) (Variables|Grabber|GetGrabberDistance))))))
        (:then_1
          (Math|Float|CompareFloat (Math|Float|Absolute(Float) _returnvalue) 0.5
            (:>
              (bind _output_get (Variables|Grabber|SetGrabberScale (Math|Float|Clamp(Float) (+ (* _returnvalue_2 _returnvalue) (Variables|Grabber|GetGrabberScale)) 0.02 1.5)))
              (Transformation|SetRelativeScale3D (Variables|Grabber|GetGrabbedObject) (Math|Vector|MakeVector _output_get _output_get _output_get)))))))))

(fn ConstructionScript
  ;[1 1 1] If in Intro hide widget set size otherwise hide
)

(fn FSoftLock
  (params (Component_Scene :type Scene%20Component%20Object%20Reference))
  (bind _returnvalue (Game|GetPlayerCameraManager 0))
  (bind _returnvalue_2 (Camera|GetCameraLocation _returnvalue))
  (bind _output_get (Variables|Default|SetLocationTarget (+ _returnvalue_2 (* (Transformation|GetActorForwardVector _returnvalue) (Variables|Default|GetWidgetDistance)))))
  (bind _output_get_2 (Variables|Default|SetLocationCurrent (Math|Vector|Lerp(Vector) (Variables|Default|GetLocationCurrent) _output_get (* (Utilities|Time|GetWorldDeltaSeconds) (Variables|Default|GetWidgetInterpSpeed)))))
  (Transformation|SetWorldLocation Component_Scene _output_get_2 false false)
  (Transformation|SetWorldRotation Component_Scene (Math|Rotator|FindLookatRotation (Transformation|GetWorldLocation Component_Scene) _returnvalue_2) false false))

(fn FDrawRayTraceControllertoCollision
  (bind _motioncontroller (Variables|Default|GetMotionController))
  (bind _tracemeshbeam (Variables|Default|GetTraceMeshBeam))
  (bind _beamthickness_0 (Variables|Trace|GetBeamThickness_0))
  (bind _beamlength_0 (Variables|Trace|GetBeamLength_0))
  (bind _returnvalue (Transformation|GetWorldLocation _motioncontroller))
  (bind _returnvalue_2 (* _beamthickness_0 0.01))
  (if (not (Variables|Default|GetEnableWidget))
    (bind _outhit (Collision|LineTraceByChannel _returnvalue (+ (* (Math|Vector|GetForwardVector _motioncontroller) (Variables|Trace|GetTraceDistance_0)) _returnvalue) "TraceTypeQuery1" false 0 "None" true "(R=0.000000,G=0.500000,B=1.000000,A=1.000000)"))
    (if (.bblockinghit _outhit)
      (Variables|Trace|SetHitActor_0 (.hitactor _outhit))
      (bind _output_get (Variables|Trace|SetBeamLengthNew_0 (* (* (/ (- (.distance _outhit) (Variables|Trace|GetBeamOriginOffset_0)) _beamlength_0) _beamlength_0) 0.01)))
      (Transformation|SetWorldScale3D _tracemeshbeam (Math|Vector|MakeVector _returnvalue_2 _returnvalue_2 _output_get))
      (else
        (Variables|Trace|SetHitActor_0 0)
        (bind _output_get_2 (Variables|Trace|SetBeamLengthNew_0 (* (Variables|Trace|GetBeamLength_0) 0.01)))
        (Transformation|SetWorldScale3D _tracemeshbeam (Math|Vector|MakeVector _returnvalue_2 _returnvalue_2 _output_get_2))))
    (Transformation|SetRelativeLocation _tracemeshbeam (Math|Vector|MakeVector (Math|Float|Absolute(Float) (+ (* (Variables|Trace|GetBeamLengthNew_0) 0.5 1e+02) (Variables|Trace|GetBeamOriginOffset_0))) 0.0 0.0) false false)))

(fn FShrinkBeam
  (Transformation|SetWorldScale3D (Variables|Default|GetTraceMeshBeam) "0, 0, 0")
  (Transformation|SetWorldScale3D (Variables|Default|GetTraceMeshEnd) "0, 0, 0"))

(fn FSetWidgetMeshing
  (bind _self self)
  (bind _widget (Variables|/Game/BluePrints/XR_Pawn.XR_Pawn_C|GetWidget _self))
  ;[1 1 1] Meshing widget and gestures widget
  (bind _returnvalue (UserInterface|CreateWidget "/Game/UI/W_01_Options_Menu.W_01_Options_Menu_C"))
  (UserInterface|SetWidget _widget _returnvalue)
  (Transformation|SetWorldScale3D _widget (Math|Conversions|ToVector(Float) (Variables|/Game/BluePrints/XR_Pawn.XR_Pawn_C|GetWidgetScale _self)))
  (return _returnvalue))

(fn FSetWidgetIntro
  (bind _self self)
  (bind _widget (Variables|/Game/BluePrints/XR_Pawn.XR_Pawn_C|GetWidget _self))
  (bind _returnvalue (UserInterface|CreateWidget "/Game/UI/W_00_Intro.W_00_Intro_C"))
  (UserInterface|SetWidget _widget 0)
  (UserInterface|SetWidget _widget _returnvalue)
  (Transformation|SetWorldScale3D _widget (Math|Conversions|ToVector(Float) (Variables|/Game/BluePrints/XR_Pawn.XR_Pawn_C|GetWidgetScale _self)))
  (return _returnvalue))

(fn FSetWidgetMenuHoverSelection
  (params (Menu :type User%20Widget%20Object%20Reference))
  ;[1 1 1] Gui Interaction Map
  (if (Variables|Default|GetEnableWidget)
    (bind _asuser_widget_parent (Utilities|Casting|CastToUser_Widget_Parent Menu))
    (Default|HoverChanged _asuser_widget_parent (Class|Actor|GetInputAxisKeyValue))))

(fn FSetMenuHoverClickEvent
  (params (Menu :type Widget%20Object%20Reference))
  (if (Variables|Default|GetEnableWidget)
    (bind _asuser_widget_parent (Utilities|Casting|CastToUser_Widget_Parent Menu))
    (Default|BtnSelected _asuser_widget_parent)))

(fn FSpawnObjectatCursor
  (bind _motioncontroller (Variables|Default|GetMotionController))
  (bind _returnvalue (Transformation|GetWorldLocation _motioncontroller))
  (bind _outhit (Collision|LineTraceByChannel _returnvalue (+ (* (Math|Vector|GetForwardVector _motioncontroller) (Variables|Trace|GetTraceDistance_0)) _returnvalue) "TraceTypeQuery1" false 0 "None" true "(R=0.000000,G=0.500000,B=1.000000,A=1.000000)"))
  (bind _returnvalue_2 (Game|SpawnActorfromClass "/Game/BluePrints/Objects/BP_Cube.BP_Cube_C" (Math|Transform|MakeTransform (+ (.location _outhit) "0,0.000000,15.000000") "0, 0, 0" "0.150000,0.150000,0.150000") "AdjustIfPossibleButAlwaysSpawn" 0 0))
  (Rendering|Material|SetMaterial (Variables|/Game/BluePrints/Objects/BP_Cube.BP_Cube_C|GetStaticMesh _returnvalue_2) 0 (Variables|Colors|GetMatBase)))

(fn FSetWidgetHelp
  (bind _self self)
  (bind _widget (Variables|/Game/BluePrints/XR_Pawn.XR_Pawn_C|GetWidget _self))
  (bind _returnvalue (UserInterface|CreateWidget "/Game/UI/W_02_Help_Menu.W_02_Help_Menu_C"))
  (UserInterface|SetWidget _widget _returnvalue)
  (Transformation|SetWorldScale3D _widget (Math|Conversions|ToVector(Float) (Variables|/Game/BluePrints/XR_Pawn.XR_Pawn_C|GetWidgetScale _self)))
  (return _returnvalue))

(fn FSetWidgetGestures
  (bind _self self)
  (bind _widget_gestures (Variables|/Game/BluePrints/XR_Pawn.XR_Pawn_C|GetWidget_Gestures _self))
  (bind _returnvalue (UserInterface|CreateWidget "/Game/UI/W_Gestures_Recognized.W_Gestures_Recognized_C"))
  (UserInterface|SetWidget _widget_gestures _returnvalue)
  (Transformation|SetWorldScale3D _widget_gestures (Math|Conversions|ToVector(Float) (Variables|/Game/BluePrints/XR_Pawn.XR_Pawn_C|GetWidgetScale _self)))
  (return _returnvalue))

(fn FLineTracefromController
  (bind _motioncontroller (Variables|Default|GetMotionController))
  (bind _returnvalue (Transformation|GetWorldLocation _motioncontroller))
  (bind (_outhit _returnvalue_2) (Collision|LineTraceForObjects _returnvalue (+ _returnvalue (* (Math|Vector|GetForwardVector _motioncontroller) 5e+02)) (Utilities|Array|MakeArray "ObjectTypeQuery4") false 0 "None"))
  (if _returnvalue_2
    (Variables|Grabber|SetGrabberDistance (.Distance (Collision|BreakHitResult _outhit))))
  (return (.HitComponent (Collision|BreakHitResult _outhit)) _returnvalue_2 (.Location (Collision|BreakHitResult _outhit))))

(fn FGrabObject
  (params (HitComponent :type Primitive%20Component%20Object%20Reference) (ObjectHit :type Boolean) (Location :type Vector))
  (Variables|Grabber|SetObjectGrabbed true)
  (if ObjectHit
    (bind _output_get (Variables|Grabber|SetGrabbedObject HitComponent))
    (Utilities|FlowControl|Sequence
      (:then_0
        (Class|PhysicsHandleComponent|GrabComponentatLocation (Variables|Default|GetPhysicsHandle) _output_get "None" Location))
      (:then_1
        (Collision|SetCollisionResponsetoChannel _output_get "ECC_Pawn" "ECR_Ignore"))
      (:then_2
        (Class|PrimitiveComponent|SetAngularDamping _output_get 1e+02))
      (:then_3
        (bind _asmesh_component (Utilities|Casting|CastToMeshComponent _output_get))
        (Rendering|Material|SetMaterial _asmesh_component 0 (Variables|Colors|GetMatSelected))))))

(fn FObjectHovered
  (params (HitComponent :type Primitive%20Component%20Object%20Reference))
  (Utilities|FlowControl|Sequence
    (:then_0
      (bind _asmesh_component (Utilities|Casting|CastToMeshComponent (Variables|Grabber|GetLastHoveredObject)))
      (Rendering|Material|SetMaterial _asmesh_component 0 (Variables|Colors|GetMatBase)))
    (:then_1
      (bind _asmesh_component_2 (Utilities|Casting|CastToMeshComponent HitComponent))
      (Rendering|Material|SetMaterial _asmesh_component_2 0 (Variables|Colors|GetMatHover)))
    (:then_2
      (Variables|Grabber|SetLastHoveredObject HitComponent))))

(fn FGestureCollision
  (params (TestLocation :type Vector))
  (bind (_outhit _returnvalue) (Class|KismetSystemLibrary|CapsuleTraceSingleforObjects "0, 0, 0" (+ TestLocation "1.000000,1.000000,1.000000") 5.0 0.0 (Utilities|Array|MakeArray "ObjectTypeQuery4") false 0 "ForDuration" true))
  (if _returnvalue
    _
    (else
      _))
  (return (.HitComponent (Collision|BreakHitResult _outhit)) _returnvalue (.Location (Collision|BreakHitResult _outhit))))

(fn FDropObject
  (Variables|Grabber|SetObjectGrabbed false)
  (Utilities|FlowControl|Sequence
    (:then_0
      (bind _asmesh_component (Utilities|Casting|CastToMeshComponent (Variables|Grabber|GetGrabbedObject)))
      (Rendering|Material|SetMaterial _asmesh_component 0 (Variables|Colors|GetMatBase)))
    (:then_1
      (Physics|Components|PhysicsHandle|ReleaseComponent (Variables|Default|GetPhysicsHandle)))
    (:then_2
      (if (== (Variables|Grabber|GetGrabbedObject) "/Game/BluePrints/Objects/BP_Cube.BP_Cube")
        (Collision|SetCollisionResponsetoChannel (Variables|Grabber|GetGrabbedObject) "ECC_Pawn" "ECR_Block")
        (else
          (Variables|Grabber|SetGrabbedObject 0))))
    (:then_3
      (Class|PrimitiveComponent|SetAllPhysicsLinearVelocity (Variables|Grabber|GetGrabbedObject) "0, 0, 0" false))
    (:then_4
      (Class|PrimitiveComponent|SetAngularDamping (Variables|Grabber|GetGrabbedObject) 0.0)
      (Variables|Grabber|SetGrabberRotation 0.0)
      (Variables|Grabber|SetGrabberScale 0.0)
      (Variables|Grabber|SetGrabbedObject 0))))