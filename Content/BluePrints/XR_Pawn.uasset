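; Player pawn for a Magic Leap XR app that drives floating menus and controller-based object interaction.
; BeginPlay picks widgets by level name; Tick lerps them toward a point ahead of the camera, facing the player.
; Right-controller input navigates menus, grabs physics objects through a PhysicsHandle, spawns cubes at trace hits and draws a beam while menus are hidden.
; Home single-click toggles the menu; double-click opens Meshing from Intro, otherwise quits.
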(event Custom|setWidget
  (bind _widget_gestures (Variables|Default|GetWidget_Gestures))
  (Utilities|FlowControl|Sequence
    (:then_0
      (if (Variables|Default|GetIsMainWidget)
        (Variables|Default|SetIsMainWidget false)
        (CallFunction|SetWidgettoHelp)
        (Transformation|SetWorldScale3D _widget_gestures "0, 0, 0")
        (else
          (Variables|Default|SetIsMainWidget true)
          (CallFunction|SetWidgettoMeshing)
          (Transformation|SetWorldScale3D _widget_gestures (Math|Conversions|ToVector(Float) (Variables|Default|GetWidgetScale))))))))

(event Custom|CustomEvent_1
  (params (GestureData :type Magic%20Leap%20Touchpad%20Gesture%20Structure%20%28by%20ref%29)))

(event Custom|WidgetSoftlock
  (params (DeltaSeconds :type Float%20%28single-precision%29))
  (bind _returnvalue (Game|GetPlayerCameraManager 0))
  (bind _widget (Variables|Default|GetWidget))
  (bind _widget_gestures (Variables|Default|GetWidget_Gestures))
  (bind _returnvalue_2 (Transformation|GetWorldLocation _widget))
  (bind _returnvalue_3 (Camera|GetCameraLocation _returnvalue))
  (bind _returnvalue_4 (Math|Rotator|FindLookatRotation _returnvalue_2 _returnvalue_3))
  ;[0 0 0] Widget Softlock. Interps between current position and positon from previous tick
  (bind _output_get (Variables|Default|SetLocationTarget (+ _returnvalue_3 (* (Transformation|GetActorForwardVector _returnvalue) (Variables|Default|GetWidgetDistance)))))
  (bind _output_get_2 (Variables|Default|SetLocationCurrent (Math|Vector|Lerp(Vector) (Variables|Default|GetLocationCurrent) _output_get (* DeltaSeconds (Variables|Default|GetWidgetInterpSpeed)))))
  (Transformation|SetWorldLocation _widget _output_get_2 false false)
  (Transformation|SetWorldRotation _widget _returnvalue_4 false false)
  (Transformation|SetWorldLocation _widget_gestures _output_get_2 false false)
  (Transformation|SetWorldRotation _widget_gestures _returnvalue_4 false false))

(event Custom|TickSetGrabLocation
  (bind _motioncontroller (Variables|Default|GetMotionController))
  ;[1 1 1] Set Grabbed Object Location
  (Physics|Components|PhysicsHandle|SetTargetLocation (Variables|Default|GetPhysicsHandle) (+ (Transformation|GetWorldLocation _motioncontroller) (* (Math|Vector|GetForwardVector _motioncontroller) (Variables|Grabber|GetGrabberDistance)))))

(event Custom|SetWidgetScale
  (bind _widget (Variables|Default|GetWidget))
  ;[1 1 1] Setup Hide show widget
  (Utilities|FlowControl|Sequence
    (:then_0
      (if (Variables|Default|GetEnableWidget)
        (Variables|Default|SetEnableWidget false)
        (Transformation|SetWorldScale3D _widget "0, 0, 0")
        (else
          (Variables|Default|SetEnableWidget true)
          (Transformation|SetWorldScale3D _widget (Math|Conversions|ToVector(Float) (Variables|Default|GetWidgetScale))))))))

(event Custom|BtnPressIntro
  ;[0 0 0] Quit Game on Home Press Right
  (Game|OpenLevel(byName) "Meshing"))

(event Custom|PickUp
  (bind _motioncontroller (Variables|Default|GetMotionController))
  (bind _returnvalue (Transformation|GetWorldLocation _motioncontroller))
  ;[1 1 1] Pickup Object
  (Variables|Grabber|SetObjectGrabbed true)
  (bind (_outhit _returnvalue_2) (Collision|LineTraceForObjects _returnvalue (+ _returnvalue (* (Math|Vector|GetForwardVector _motioncontroller) 5e+02)) (Utilities|Array|MakeArray "ObjectTypeQuery4") false 0 "Persistent"))
  (if _returnvalue_2
    (Variables|Grabber|SetGrabberDistance (.Distance (Collision|BreakHitResult _outhit)))
    (bind _output_get (Variables|Grabber|SetGrabbedObject (.HitComponent (Collision|BreakHitResult _outhit))))
    (Class|PhysicsHandleComponent|GrabComponentatLocation (Variables|Default|GetPhysicsHandle) _output_get "None" (.Location (Collision|BreakHitResult _outhit)))
    (Collision|SetCollisionResponsetoChannel _output_get "ECC_Pawn" "ECR_Ignore")
    (Class|PrimitiveComponent|SetAngularDamping _output_get 1e+01)))

(event Custom|Set%20Widget%20to%20Help
  ;[1 1 1] Set up menu btn selection
  (bind _returnvalue (CallFunction|FSetWidgetHelp)))

(event Custom|Drop
  (bind _grabbedobject (Variables|Grabber|GetGrabbedObject))
  ;[1 1 1] Drop Object
  (Variables|Grabber|SetObjectGrabbed false)
  (Physics|Components|PhysicsHandle|ReleaseComponent (Variables|Default|GetPhysicsHandle))
  (if (== _grabbedobject "/Game/BluePrints/Objects/BP_Cube.BP_Cube")
    (Collision|SetCollisionResponsetoChannel _grabbedobject "ECC_Pawn" "ECR_Block")
    (Class|PrimitiveComponent|SetAllPhysicsLinearVelocity _grabbedobject "0, 0, 0" false)
    (Utilities|FlowControl|Delay 0.2)
    (Class|PrimitiveComponent|SetAngularDamping _grabbedobject 0.0)
    (Variables|Grabber|SetGrabberRotation 0.0)
    (Variables|Grabber|SetGrabberScale 0.0)))

(event Custom|Set%20Widget%20to%20Intro
  ;[1 1 1] Set up menu btn selection
  (bind _intro (CallFunction|FSetWidgetIntro)))

(event Custom|Set%20Widget%20toMeshing
  ;[1 1 1] Set up menu btn selection
  (bind _meshing_menu (CallFunction|FSetWidgetMeshing)))

(event EventBeginPlay
  ;[1 1 1] Begin Play
  (bind _asbp_game_mode (Utilities|Casting|CastToBP_GameMode (Game|GetGameMode)))
  (bind _output_get (Variables|/Game/Maps/BP_GameMode.BP_GameMode_C|SetXR_Pawn _asbp_game_mode self))
  (Utilities|FlowControl|Sequence
    (:then_0
      (Pawn|Possess (Game|GetPlayerController 0) _output_get)
      (Utilities|IsValid (Variables|XR_Pawn_C|GetMotionController _output_get)
        (:Is%20Valid
          (Variables|/Script/HeadMountedDisplay.MotionControllerComponent|SetMotionSource (Variables|XR_Pawn_C|GetMotionController _output_get) "Right"))))
    (:then_1
      (bind _returnvalue (Game|GetCurrentLevelName true))
      (switch string _returnvalue
        (:Intro
          (CallFunction|SetWidgettoIntro))
        (:Meshing
          (Utilities|FlowControl|Sequence
            (:then_0
              (CallFunction|SetWidgettoMeshing)
              (Variables|Default|SetIsMainWidget true))
            (:then_1
              (CallFunction|FSetWidgetGestures))))))))

(event EventTick
  (params (DeltaSeconds :type Float%20%28single-precision%29))
  ;[1 0 1] Tick
  (CallFunction|FSoftLock (Variables|Default|GetWidget))
  (CallFunction|FSoftLock (Variables|Default|GetWidget_Gestures))
  (Utilities|FlowControl|Sequence
    (:then_0
      (if (Variables|Grabber|GetObjectGrabbed)
        (CallFunction|TickSetGrabLocation)))
    (:then_1
      (if (Variables|Default|GetTriggerPressed)
        (CallFunction|FDrawRayTraceControllertoCollision)))))

(event Input|KeyboardEvents|MotionControllerRightTrigger
  (params (Key :type Key%20Structure))
  ;[1 1 1] Grabber Input Binding
  (:Pressed
    (CallFunction|PickUp))
  (:Released
    (CallFunction|Drop)))

(event Input|KeyboardEvents|MotionControllerRightThumbstick
  (params (Key :type Key%20Structure))
  ;[1 1 1] Set up menu btn selection
  (:Pressed
    (if (not (Variables|Default|GetIsMainWidget))
      (CallFunction|FSetWidgetMenuHoverSelection (stale Custom|Set%20Widget%20to%20Help _returnvalue))
      (Class|MagicLeapControllerFunctionLibrary|PlayHapticPattern "Right" "None" "Low"))))

(event Input|KeyboardEvents|MotionControllerRightThumbstick
  (params (Key :type Key%20Structure))
  ;[1 1 1] Set up menu btn selection
  (:Pressed
    (CallFunction|FSetWidgetMenuHoverSelection (stale Custom|Set%20Widget%20to%20Intro _intro))
    (Class|MagicLeapControllerFunctionLibrary|PlayHapticPattern "Right" "None" "Low")))

(event Input|KeyboardEvents|MotionControllerRightThumbstick
  (params (Key :type Key%20Structure))
  ;[1 1 1] Set up menu btn selection
  (:Pressed
    (if (Variables|Default|GetIsMainWidget)
      (CallFunction|FSetWidgetMenuHoverSelection (stale Custom|Set%20Widget%20toMeshing _meshing_menu))
      (Class|MagicLeapControllerFunctionLibrary|PlayHapticPattern "Right" "None" "Low"))))

(event Input|KeyboardEvents|MotionControllerRightTrigger
  (params (Key :type Key%20Structure))
  ;[1 1 1] Set up menu btn selection
  (:Pressed
    (if (Variables|Default|GetIsMainWidget)
      (CallFunction|FSetMenuHoverClickEvent (stale Custom|Set%20Widget%20toMeshing _meshing_menu))
      (Class|MagicLeapControllerFunctionLibrary|PlayHapticPattern "Right" "None" "Low"))))

(event Input|KeyboardEvents|MagicLeapRightHomeButton
  (params (Key :type Key%20Structure))
  ;[1 1 1] Haptics
  (:Pressed
    (Audio|PlaySound2D "/Game/Sounds/ui_confirm_short.ui_confirm_short" 1.0 1.0 0.0 0 0)
    (Class|MagicLeapControllerFunctionLibrary|PlayHapticPattern "Right" "ForceDown" "Low")))

(event Input|KeyboardEvents|MotionControllerRightShoulder
  (params (Key :type Key%20Structure))
  ;[1 1 1] Haptics
  (:Pressed
    (Audio|PlaySound2D "/Game/Sounds/ui_confirm_short.ui_confirm_short" 1.0 1.0 0.0 0 0)
    (Class|MagicLeapControllerFunctionLibrary|PlayHapticPattern "Right" "ForceDown" "Low")))

(event Input|KeyboardEvents|MotionControllerRightTrigger
  (params (Key :type Key%20Structure))
  ;[1 1 1] Set up menu btn selection
  (:Pressed
    (CallFunction|FSetMenuHoverClickEvent (stale Custom|Set%20Widget%20to%20Intro _intro))
    (Class|MagicLeapControllerFunctionLibrary|PlayHapticPattern "Right" "None" "Low")))

(event Input|KeyboardEvents|MotionControllerRightShoulder
  (params (Key :type Key%20Structure))
  ;[1 1 1] Spawn Object
  (:Pressed
    (CallFunction|FSpawnObjectatCursor)))

(event Input|KeyboardEvents|MotionControllerRightTrigger
  (params (Key :type Key%20Structure))
  ;[1 1 1] Draw Beam
  (:Pressed
    (Variables|Default|SetTriggerPressed true))
  (:Released
    (Variables|Default|SetTriggerPressed false)
    (CallFunction|FShrinkBeam)))

(event Input|KeyboardEvents|MotionControllerRightTrigger
  (params (Key :type Key%20Structure))
  ;[1 1 1] Set up menu btn selection
  (:Pressed
    (if (not (Variables|Default|GetIsMainWidget))
      (CallFunction|FSetMenuHoverClickEvent (stale Custom|Set%20Widget%20to%20Help _returnvalue))
      (Class|MagicLeapControllerFunctionLibrary|PlayHapticPattern "Right" "None" "Low"))))

(event Input|KeyboardEvents|MagicLeapRightHomeButton
  (params (Key :type Key%20Structure))
  ;[0 0 0] Quit Game on Home Press Right
  (:Pressed
    (Utilities|DetectDoubleClick
      (:Double%20Click
        (bind _returnvalue (Game|GetCurrentLevelName true))
        (if (Utilities|Enum|Equal(Enum) _returnvalue "Intro")
          (Game|OpenLevel(byName) "Meshing")
          (else
            (Game|QuitGame 0 "Quit" false))))
      (:Single%20Click
        (CallFunction|SetWidgetScale)))))

(event Input|KeyboardEvents|MotionControllerRightThumbstick
  (params (Key :type Key%20Structure))
  (bind _returnvalue (Class|Actor|GetInputAxisKeyValue))
  (bind _returnvalue_2 (Class|Actor|GetInputAxisKeyValue))
  (bind _returnvalue_3 (Class|Actor|GetInputAxisKeyValue))
  ;[1 1 1] Grabber Scale, Extend
  (:Pressed
    (if (Variables|Grabber|GetObjectGrabbed)
      (Utilities|FlowControl|Sequence
        (:then_0
          (Math|Float|CompareFloat (Math|Float|Absolute(Float) _returnvalue_3) 0.5
            (:>
              (Variables|Grabber|SetGrabberDistance (+ (* _returnvalue_3 (* _returnvalue_2 2e+02)) (Variables|Grabber|GetGrabberDistance))))))
        (:then_1
          (Math|Float|CompareFloat (Math|Float|Absolute(Float) _returnvalue) 0.5
            (:>
              (Variables|Grabber|SetGrabberScale (+ (* _returnvalue_2 _returnvalue) (Variables|Grabber|GetGrabberScale)))
              (Transformation|SetRelativeScale3D (Variables|Grabber|GetGrabbedObject) (Math|Vector|MakeVector (Variables|Grabber|GetGrabberScale) (Variables|Grabber|GetGrabberScale) (Variables|Grabber|GetGrabberScale))))))))))

(fn ConstructionScript
  ;[1 1 1] If in Intro hide widget set size otherwise hide
)

(fn FSoftLock
  (params (Component_Scene :type Scene%20Component%20Object%20Reference))
  (bind _returnvalue (Game|GetPlayerCameraManager 0))
  (bind _returnvalue_2 (Camera|GetCameraLocation _returnvalue))
  (bind _output_get (Variables|Default|SetLocationTarget (+ _returnvalue_2 (* (Transformation|GetActorForwardVector _returnvalue) (Variables|Default|GetWidgetDistance)))))
  (bind _output_get_2 (Variables|Default|SetLocationCurrent (Math|Vector|Lerp(Vector) (Variables|Default|GetLocationCurrent) _output_get (* (Utilities|Time|GetWorldDeltaSeconds) (Variables|Default|GetWidgetInterpSpeed)))))
  (Transformation|SetWorldLocation Component_Scene _output_get_2 false false)
  (Transformation|SetWorldRotation Component_Scene (Math|Rotator|FindLookatRotation (Transformation|GetWorldLocation Component_Scene) _returnvalue_2) false false))

(fn FDrawRayTraceControllertoCollision
  (bind _motioncontroller (Variables|Default|GetMotionController))
  (bind _tracemeshbeam (Variables|Default|GetTraceMeshBeam))
  (bind _beamthickness_0 (Variables|Trace|GetBeamThickness_0))
  (bind _beamlength_0 (Variables|Trace|GetBeamLength_0))
  (bind _tracemeshend (Variables|Default|GetTraceMeshEnd))
  (bind _returnvalue (Transformation|GetWorldLocation _motioncontroller))
  (bind _returnvalue_2 (* _beamthickness_0 0.01))
  (if (not (Variables|Default|GetEnableWidget))
    (bind _outhit (Collision|LineTraceByChannel _returnvalue (+ (* (Math|Vector|GetForwardVector _motioncontroller) (Variables|Trace|GetTraceDistance_0)) _returnvalue) "TraceTypeQuery1" false 0 "None" true "(R=0.000000,G=0.500000,B=1.000000,A=1.000000)"))
    (if (.bblockinghit _outhit)
      (Variables|Trace|SetHitActor_0 (.hitactor _outhit))
      (bind _output_get (Variables|Trace|SetBeamLengthNew_0 (* (* (/ (- (.distance _outhit) (Variables|Trace|GetBeamOriginOffset_0)) _beamlength_0) _beamlength_0) 0.01)))
      (Transformation|SetWorldScale3D _tracemeshbeam (Math|Vector|MakeVector _returnvalue_2 _returnvalue_2 _output_get))
      (Development|SetHiddeninGame _tracemeshend false false)
      (else
        (Variables|Trace|SetHitActor_0 0)
        (bind _output_get_2 (Variables|Trace|SetBeamLengthNew_0 (* (Variables|Trace|GetBeamLength_0) 0.01)))
        (Transformation|SetWorldScale3D _tracemeshbeam (Math|Vector|MakeVector _returnvalue_2 _returnvalue_2 _output_get_2))
        (Development|SetHiddeninGame _tracemeshend false false)))
    (Transformation|SetRelativeLocation _tracemeshbeam (Math|Vector|MakeVector (Math|Float|Absolute(Float) (+ (* (Variables|Trace|GetBeamLengthNew_0) 0.5 1e+02) (Variables|Trace|GetBeamOriginOffset_0))) 0.0 0.0) false false)
    (Transformation|SetWorldLocationAndRotation (Variables|Default|GetTraceMeshEnd) (.location _outhit) (Math|Rotator|MakeRotator (.Roll (Math|Rotator|BreakRotator (Math|Conversions|RotationFromXVector (.normal _outhit)))) (+ (.Pitch (Math|Rotator|BreakRotator (Math|Conversions|RotationFromXVector (.normal _outhit)))) 9e+01) (.Yaw (Math|Rotator|BreakRotator (Math|Conversions|RotationFromXVector (.normal _outhit))))) false false)))

(fn FShrinkBeam
  (Transformation|SetWorldScale3D (Variables|Default|GetTraceMeshBeam) "0, 0, 0")
  (Transformation|SetWorldScale3D (Variables|Default|GetTraceMeshEnd) "0, 0, 0"))

(fn FSetWidgetMeshing
  (bind _self self)
  (bind _widget (Variables|XR_Pawn_C|GetWidget _self))
  ;[1 1 1] Meshing widget and gestures widget
  (bind _returnvalue (UserInterface|CreateWidget "/Game/UI/W_01_Options_Menu.W_01_Options_Menu_C"))
  (UserInterface|SetWidget _widget _returnvalue)
  (Transformation|SetWorldScale3D _widget (Math|Conversions|ToVector(Float) (Variables|XR_Pawn_C|GetWidgetScale _self)))
  (return _returnvalue))

(fn FSetWidgetIntro
  (bind _self self)
  (bind _widget (Variables|XR_Pawn_C|GetWidget _self))
  (bind _returnvalue (UserInterface|CreateWidget "/Game/UI/W_00_Intro.W_00_Intro_C"))
  (UserInterface|SetWidget _widget 0)
  (UserInterface|SetWidget _widget _returnvalue)
  (Transformation|SetWorldScale3D _widget (Math|Conversions|ToVector(Float) (Variables|XR_Pawn_C|GetWidgetScale _self)))
  (return _returnvalue))

(fn FSetWidgetMenuHoverSelection
  (params (Menu :type User%20Widget%20Object%20Reference))
  ;[1 1 1] Gui Interaction Map
  (if (Variables|Default|GetEnableWidget)
    (bind _asuser_widget_parent (Utilities|Casting|CastToUser_Widget_Parent Menu))
    (Default|HoverChanged _asuser_widget_parent (Class|Actor|GetInputAxisKeyValue))))

(fn FSetMenuHoverClickEvent
  (params (Menu :type Widget%20Object%20Reference))
  (if (Variables|Default|GetEnableWidget)
    (bind _asuser_widget_parent (Utilities|Casting|CastToUser_Widget_Parent Menu))
    (Default|BtnSelected _asuser_widget_parent)))

(fn FSpawnObjectatCursor
  (bind _motioncontroller (Variables|Default|GetMotionController))
  (bind _returnvalue (Transformation|GetWorldLocation _motioncontroller))
  (bind _outhit (Collision|LineTraceByChannel _returnvalue (+ (* (Math|Vector|GetForwardVector _motioncontroller) (Variables|Trace|GetTraceDistance_0)) _returnvalue) "TraceTypeQuery1" false 0 "None" true "(R=0.000000,G=0.500000,B=1.000000,A=1.000000)"))
  (Game|SpawnActorfromClass "/Game/BluePrints/Objects/BP_Cube.BP_Cube_C" (Math|Transform|MakeTransform (.location _outhit) "0, 0, 0" "0.150000,0.150000,0.150000") "AdjustIfPossibleButAlwaysSpawn" 0 0))

(fn FSetWidgetHelp
  (bind _self self)
  (bind _widget (Variables|XR_Pawn_C|GetWidget _self))
  (bind _returnvalue (UserInterface|CreateWidget "/Game/UI/W_02_Help_Menu.W_02_Help_Menu_C"))
  (UserInterface|SetWidget _widget _returnvalue)
  (Transformation|SetWorldScale3D _widget (Math|Conversions|ToVector(Float) (Variables|XR_Pawn_C|GetWidgetScale _self)))
  (return _returnvalue))

(fn FSetWidgetGestures
  (bind _self self)
  (bind _widget_gestures (Variables|XR_Pawn_C|GetWidget_Gestures _self))
  (bind _returnvalue (UserInterface|CreateWidget "/Game/UI/W_Gestures_Recognized.W_Gestures_Recognized_C"))
  (UserInterface|SetWidget _widget_gestures _returnvalue)
  (Transformation|SetWorldScale3D _widget_gestures (Math|Conversions|ToVector(Float) (Variables|XR_Pawn_C|GetWidgetScale _self)))
  (return _returnvalue))