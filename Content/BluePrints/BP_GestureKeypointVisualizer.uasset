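; BP_GestureKeypointVisualizer shows or hides tagged hand keypoint motion controller components on the XR pawn.
; After a short BeginPlay delay, it caches left and right components and binds to the game mode's GestureReader.
; Detected gestures set per-hand active flags, which are ANDed with show flags from SetShowKeypoints to drive visibility.
; Both refresh calls pass Hand 0, so the right-side result targets the same hand as the left.
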(event Custom|OnGestureDetected
  (params (Gesture :type EHandTrackingGesture%20Enum :default "Finger") (Hand :type E_HandType%20Enum :default "NewEnumerator0"))
  ;[1 0.6771 0.6771] Show or hide keypoints based on detected hand state
  (Gestures|CheckValidGesture Gesture Hand))

(event EventBeginPlay
  (Utilities|FlowControl|Delay 0.2)
  (bind _asbp_game_mode (Utilities|Casting|CastToBP_GameMode (Game|GetGameMode)))
  ;[0.165 1 0.1379] Initialize
  (EventDispatchers|BindEventtoOnGestureDetected (Variables|/Game/Maps/BP_GameMode.BP_GameMode_C|GetGestureReader _asbp_game_mode) (delegate Custom|OnGestureDetected))
  (Variables|Components|SetLeftKeypoints (Actor|GetComponentsbyTag (Variables|/Game/Maps/BP_GameMode.BP_GameMode_C|GetXR_Pawn _asbp_game_mode) "/Script/HeadMountedDisplay.MotionControllerComponent" "Left Keypoints"))
  (Variables|Components|SetRightKeypoints (Actor|GetComponentsbyTag (Variables|/Game/Maps/BP_GameMode.BP_GameMode_C|GetXR_Pawn _asbp_game_mode) "/Script/HeadMountedDisplay.MotionControllerComponent" "Right Keypoints")))

(fn ConstructionScript)

(fn CheckValidGesture
  (params (Gesture :type EHandTrackingGesture%20Enum :default "Finger") (Hand :type E_HandType%20Enum :default "NewEnumerator0"))
  (Utilities|FlowControl|Sequence
    (:then_0
      ;[1 1 1] Only show keypoints when hand is detected
      (LocalVariables|SetIsValidGesture (Utilities|Enum|NotEqual(Enum) Gesture "NoHand")))
    (:then_1
      (switch Utilities|FlowControl|Switch|SwitchonE_HandType Hand
        (:NewEnumerator0
          (Variables|Gestures|SetLeftKeypointsActive (LocalVariables|GetIsValidGesture)))
        (:NewEnumerator1
          (Variables|Gestures|SetRightKeypointsActive (LocalVariables|GetIsValidGesture)))
        (:NewEnumerator2
          (Variables|Gestures|SetLeftKeypointsActive (LocalVariables|GetIsValidGesture))
          (Variables|Gestures|SetRightKeypointsActive (LocalVariables|GetIsValidGesture)))))
    (:then_2
      (Gestures|RefreshKeypointsVisible))))

(fn SetShowKeypoints
  (params (Hand :type Byte) (Visible :type Boolean))
  (Utilities|FlowControl|Sequence
    (:then_0
      (switch Utilities|FlowControl|Switch|Switchon Hand
        (:NewEnumerator0
          (Variables|Gestures|SetShowLeftKeypoints Visible))
        (:NewEnumerator1
          (Variables|Gestures|SetShowRightKeypoints Visible))
        (:NewEnumerator2
          (Variables|Gestures|SetShowLeftKeypoints Visible)
          (Variables|Gestures|SetShowRightKeypoints Visible))))
    (:then_1
      (Gestures|RefreshKeypointsVisible))))

(fn SetKeypointsVisible
  (params (Hand :type Byte) (Visible :type Boolean))
  (bind _returnvalue (not Visible))
  (switch Utilities|FlowControl|Switch|Switchon Hand
    (:NewEnumerator0
      (for _array_element (Variables|Components|GetLeftKeypoints)
        (Development|SetHiddeninGame _array_element _returnvalue true)))
    (:NewEnumerator1
      (for _array_element_2 (Variables|Components|GetRightKeypoints)
        (Development|SetHiddeninGame _array_element_2 _returnvalue true)))))

(fn RefreshKeypointsVisible
  (Utilities|FlowControl|Sequence
    (:then_0
      (Gestures|SetKeypointsVisible 0 (and (Variables|Gestures|GetShowLeftKeypoints) (Variables|Gestures|GetLeftKeypointsActive))))
    (:then_1
      (Gestures|SetKeypointsVisible 0 (and (Variables|Gestures|GetShowRightKeypoints) (Variables|Gestures|GetRightKeypointsActive))))))