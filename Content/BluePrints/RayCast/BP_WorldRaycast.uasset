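; Raycast actor that queries the world asynchronously from its location and orientation, using its width, height and horizontal FOV.
; A bound request event clears AutoCast and sends the query; the result callback sets AutoCast again and records hit state and confidence.
; Observed or unobserved hits with positive confidence become standard HitResults, other outcomes become invalid hits, and both paths broadcast that the raycast finished.
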(event Custom|WorldRaycastRequest
  ;[0 0.2656 0.2656] World Raycast
  (Variables|Default|SetAutoCast false)
  (bind _returnvalue (Class|RaycastComponent|RequestRaycast (Variables|Default|GetWorldRaycast) (Utilities|Struct|MakeRaycastQueryParams (Transformation|GetActorLocation) (Transformation|GetActorForwardVector) (Transformation|GetActorUpVector) (Variables|WorldRaycastSettings|GetWidth) (Variables|WorldRaycastSettings|GetHeight) (Variables|WorldRaycastSettings|GetHorizontalFOVDegrees) (Variables|WorldRaycastSettings|GetCollideWithUnobserved)) (delegate Custom|OnWorldRaycastResult)))
  (if (not _returnvalue)
    ;;[1 1 1] No Hit
    (Variables|Default|SetHitResult "")
    (Variables|Default|SetIsValidHit false)
    (Default|CallOnWorldRaycastFinished)))

(event Custom|OnWorldRaycastResult
  (params (HitResult :type Raycast%20Hit%20Result%20Structure))
  (bind (_hitstate _hitpoint _normal _confidence) (Utilities|Struct|BreakRaycastHitResult HitResult))
  ;[0 0.2656 0.2656] World Raycast
  (Variables|Default|SetHitState _hitstate)
  (Variables|Default|SetConfidence _confidence)
  (Variables|Default|SetAutoCast true)
  (switch Utilities|FlowControl|Switch|SwitchonERaycastResultState _hitstate
    (:RequestFailed
      ;;[1 1 1] No Hit
      (Variables|Default|SetHitResult "" :!label _label)
      (Variables|Default|SetIsValidHit false))
    (:NoCollision
      (goto _label))
    (:HitUnobserved
      (Variables|Default|SetIsObservedHit false)
      (if (> _confidence 0.0) :!label _label_2
        ;;[0.1277 1 0.2754] Hit
        (Variables|Default|SetHitResult (Collision|MakeHitResult true false 0.0 0.0 _hitpoint _hitpoint _normal _normal 0 0))
        (Variables|Default|SetIsValidHit true)
        (else
          (goto _label))))
    (:HitObserved
      (Variables|Default|SetIsObservedHit true)
      (goto _label_2)))
  (Default|CallOnWorldRaycastFinished))

(event EventTick
  (params (DeltaSeconds :type Float%20%28single-precision%29))
  ;[1 0.7294 0.3137] Tick
  (|CallParentFunction DeltaSeconds))

(event EventBeginPlay
  ;[0.1647 1 0.1373] Initialize
  (EventDispatchers|BindEventtoRequestRaycast (delegate Custom|WorldRaycastRequest)))

(fn ConstructionScript
  (|CallParentFunction))