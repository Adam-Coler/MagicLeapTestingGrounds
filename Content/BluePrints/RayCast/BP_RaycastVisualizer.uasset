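; Cursor actor that visualizes the result of a referenced Raycast, apparently used for gaze.
; Each tick it snaps to the hit point and normal, or to the ray's default end when nothing is hit.
; The cursor material distinguishes observed hits from unobserved or missing ones, and its scale can grow at close range.
; SetHidden toggles visibility, ticking and the raycast together.
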(event EventTick
  (params (DeltaSeconds :type Float%20%28single-precision%29))
  (bind _raycast (Variables|RaycastReference|GetRaycast))
  (bind _raycast_2 (Variables|RaycastReference|GetRaycast))
  (bind _hitresult (Variables|/Game/BluePrints/RayCast/BP_BaseRaycast.BP_BaseRaycast_C|GetHitResult _raycast))
  (bind (_bblockinghit _binitialoverlap _time _distance _location _impactpoint _normal _impactnormal) (Collision|BreakHitResult _hitresult))
  ;[1 0.7294 0.3137] Tick
  (CallFunction|ScaleifClose)
  (Utilities|IsValid _raycast_2
    (:Is%20Valid
      (if (Default|HitIsValid _raycast_2)
        ;;[1 1 1] Match Gaze Hit Location/Normal
        (Transformation|SetActorLocationAndRotation _impactpoint (Math|Conversions|RotationFromXVector _impactnormal))
        (if (Default|HitIsObserved (Variables|RaycastReference|GetRaycast))
          (Rendering|Material|SetMaterial (Variables|Default|GetCursor) 0 (Variables|VisualizerSettings|GetInitialMaterial))
          (else
            (Rendering|Material|SetMaterial (Variables|Default|GetCursor) 0 0) ; Unobserved hits get a yellow cursor
          ))
        (else
          ;;[1 1 1] Set Location to Default End Position and static rotation If no Hit
          (Transformation|SetActorLocationAndRotation (Default|GetDefaultEndPosition (Variables|RaycastReference|GetRaycast)) (Transformation|GetWorldRotation (Variables|/Script/Engine.Actor|GetRootComponent (Variables|RaycastReference|GetRaycast))))
          (Rendering|Material|SetMaterial (Variables|Default|GetCursor) 0 0))))))

(event EventBeginPlay
  ;[0.1647 1 0.1373] Initialize
  (Variables|VisualizerSettings|SetInitialMaterial (Rendering|Material|GetMaterial (Variables|Default|GetCursor) 0)))

(fn ConstructionScript)

(fn GetHitLocation
  (return (Default|GetHitLocation (Variables|RaycastReference|GetRaycast))))

(fn ScaleifClose
  (bind _raycast (Variables|RaycastReference|GetRaycast))
  (bind _scalemultiplier (Variables|VisualizerSettings|GetScaleMultiplier))
  (bind _minimumscaledistance (Variables|VisualizerSettings|GetMinimumScaleDistance))
  (bind _distance (Default|GetHitDistance _raycast))
  (bind _returnvalue (- _minimumscaledistance _distance))
  (bind _returnvalue_2 (* _returnvalue _scalemultiplier))
  (bind _returnvalue_3 (Math|Float|Max(Float) _returnvalue_2 1.0))
  (if (Variables|VisualizerSettings|GetScaleWhenClose)
    (if (<= (Default|GetHitDistance (Variables|RaycastReference|GetRaycast)) (Variables|VisualizerSettings|GetMinimumScaleDistance))
      ;[1 1 1] Scale Up when Close
      (Transformation|SetRelativeScale3D (Variables|Default|GetCursor) (Math|Vector|MakeVector _returnvalue_3 _returnvalue_3 _returnvalue_3))
      (else
        (Transformation|SetRelativeScale3D (Variables|Default|GetCursor) "1.000000,1.000000,1.000000")))))

(fn SetHidden
  (params (Hidden :type Boolean))
  (bind _returnvalue (not Hidden))
  (Rendering|SetVisibility (Variables|Default|GetRoot) _returnvalue true)
  (Rendering|SetActorHiddenInGame Hidden)
  (Actor|Tick|SetActorTickEnabled self _returnvalue)
  (Default|Toggle (Variables|RaycastReference|GetRaycast) _returnvalue))