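; Magic Leap XR pawn with a controller laser pointer, head-following UI widgets and touchpad gesture input.
; Tick lerps both widgets toward a camera-forward point and resizes the laser and its hit dot from a line trace.
; A second trace beam updates during touchpad gestures and collapses when they end.
; Trigger clicks widgets, bumper toggles the main widget with haptics, Home quits, and an intro button event opens the Meshing level.
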(event OnTouchpadGestureStart(TouchpadGestures)
  (params (GestureData :type Magic%20Leap%20Touchpad%20Gesture%20Structure%20%28by%20ref%29))
  (Variables|Default|SetGesturePadTouched true))

(event OnTouchpadGestureEnd(TouchpadGestures)
  (params (GestureData :type Magic%20Leap%20Touchpad%20Gesture%20Structure%20%28by%20ref%29))
  (CallFunction|FShrinkBeam)
  (Variables|Default|SetGesturePadTouched false))

(event Custom|WidgetSoftlock
  (params (DeltaSeconds :type Float%20%28single-precision%29))
  (bind _returnvalue (Game|GetPlayerCameraManager 0))
  (bind _widget_gestures (Variables|Default|GetWidget_Gestures))
  (bind _widget (Variables|Default|GetWidget))
  (bind _returnvalue_2 (Transformation|GetWorldLocation _widget))
  (bind _returnvalue_3 (Camera|GetCameraLocation _returnvalue))
  (bind _returnvalue_4 (Math|Rotator|FindLookatRotation _returnvalue_2 _returnvalue_3))
  ;[0 0 0] Widget Softlock. Interps between current position and positon from previous tick
  (bind _output_get (Variables|Default|SetLocationTarget (+ _returnvalue_3 (* (Transformation|GetActorForwardVector _returnvalue) (Variables|Default|GetWidgetDistance)))))
  (bind _output_get_2 (Variables|Default|SetLocationCurrent (Math|Vector|Lerp(Vector) (Variables|Default|GetLocationCurrent) _output_get (* DeltaSeconds (Variables|Default|GetWidgetInterpSpeed)))))
  (Transformation|SetWorldLocation _widget _output_get_2 false false)
  (Transformation|SetWorldRotation _widget _returnvalue_4 false false)
  (Transformation|SetWorldLocation _widget_gestures _output_get_2 false false)
  (Transformation|SetWorldRotation _widget_gestures _returnvalue_4 false false))

(event Custom|ButtonPressIntro
  (params (ScreenNumber :type Integer))
  ;[1 1 1] On Intro Button CLick (Enum with levels in future) Or use different event per button
  (switch int ScreenNumber
    (:0
      (Game|OpenLevel(byName) "Meshing"))))

(event EventBeginPlay
  (CallFunction|FLaserPointerConstruction)
  (Components|Activation|Activate (Variables|Default|GetTouchpadGestures) false)
  (CallFunction|FConstructTraceBeam))

(event EventTick
  (params (DeltaSeconds :type Float%20%28single-precision%29))
  ;[1 0 1] Tick
  (CallFunction|FSoftLock (Variables|Default|GetWidget))
  (CallFunction|FSoftLock (Variables|Default|GetWidget_Gestures))
  (CallFunction|FLaserPointer)
  (if (Variables|Default|GetGesturePadTouched)
    (CallFunction|FDrawRayTraceControllertoCollision)))

(event Input|KeyboardEvents|MagicLeapRightHomeButton
  (params (Key :type Key%20Structure))
  ;[0 0 0] Quit Game on Home Press Right
  (:Pressed
    (Game|QuitGame 0 "Quit" false)))

(event Input|KeyboardEvents|MotionControllerRightTrigger
  (params (Key :type Key%20Structure))
  ;[1 1 1] Haptics
)

(event Input|KeyboardEvents|MagicLeapRightHomeButton
  (params (Key :type Key%20Structure))
  ;[1 1 1] Haptics
  (:Pressed
    (Audio|PlaySound2D "/Game/Sounds/ui_confirm_short.ui_confirm_short" 1.0 1.0 0.0 0 0)
    (Class|MagicLeapControllerFunctionLibrary|PlayHapticPattern "Right" "ForceDown" "Low")))

(event Input|KeyboardEvents|MotionControllerRightShoulder
  (params (Key :type Key%20Structure))
  ;[1 1 1] Haptics
  (:Pressed
    (Audio|PlaySound2D "/Game/Sounds/ui_confirm_short.ui_confirm_short" 1.0 1.0 0.0 0 0)
    (Class|MagicLeapControllerFunctionLibrary|PlayHapticPattern "Right" "ForceDown" "Low")))

(event Input|KeyboardEvents|MotionControllerRightTrigger
  (params (Key :type Key%20Structure))
  (bind _widgetinteraction (Variables|Default|GetWidgetInteraction))
  ;[0 0 0] Pointer Widget Interaction Mapping
  (:Pressed
    (Class|WidgetInteractionComponent|PressPointerKey _widgetinteraction "LeftMouseButton"))
  (:Released
    (Class|WidgetInteractionComponent|ReleasePointerKey _widgetinteraction "LeftMouseButton")))

(event Input|KeyboardEvents|MotionControllerRightShoulder
  (params (Key :type Key%20Structure))
  (bind _widget (Variables|Default|GetWidget))
  ;[1 1 1] Setup Hide show widget on bumper press
  (:Pressed
    (Utilities|FlowControl|Sequence
      (:then_0
        (if (Variables|Default|GetEnableWidget)
          (Variables|Default|SetEnableWidget false)
          (else
            (Variables|Default|SetEnableWidget true))))
      (:then_1
        (if (Variables|Default|GetEnableWidget)
          (Transformation|SetWorldScale3D _widget (Math|Conversions|ToVector(Float) (Variables|Default|GetWidgetScale)))
          (else
            (Transformation|SetWorldScale3D _widget "0, 0, 0")))))))

(fn ConstructionScript
  ;[1 1 1] If in Intro hide widget set size otherwise hide
)

(fn FLaserPointerConstruction
  (bind _beammesh (Variables|Default|GetBeamMesh))
  (bind _beamlength (Variables|Pointer|GetBeamLength))
  (bind _beamthickness (Variables|Pointer|GetBeamThickness))
  (bind _returnvalue (* _beamthickness 0.01))
  (bind _returnvalue_2 (* _beamlength 0.01))
  (Utilities|FlowControl|Sequence
    (:then_0
      (Transformation|SetWorldScale3D _beammesh (Math|Vector|MakeVector _returnvalue _returnvalue _returnvalue_2))
      (Transformation|SetRelativeLocation _beammesh (Math|Vector|MakeVector (Math|Float|Absolute(Float) (+ (* _beamlength 0.5) (* (Variables|Pointer|GetBeamOriginOffset) 1.0))) 0.0 0.0) false false)
      (Transformation|SetWorldScale3D (Variables|Default|GetDotMesh) (Math|Conversions|ToVector(Float) (* (Variables|Pointer|GetDotSize) 0.01))))
    (:then_1
      (bind _returnvalue_3 (Rendering|Material|CreateDynamicMaterialInstance (Variables|Default|GetBeamMesh) 0 "/Game/ToolsR1/LaserPointerTool/M_Laser.M_Laser" "None" :!class /Script/Engine.PrimitiveComponent))
      (bind _output_get (Variables|Pointer|SetBeamMaterial _returnvalue_3))
      (Rendering|Material|SetScalarParameterValue _output_get "GlobalTiling" _returnvalue_2 :!class /Script/Engine.MaterialInstanceDynamic)
      (Rendering|Material|SetScalarParameterValue _output_get "GradientFalloffUVs" (/ _returnvalue_2 (* (Variables|Pointer|GetBeamFadeLength) 0.01)) :!class /Script/Engine.MaterialInstanceDynamic)
      (Rendering|Material|SetVectorParameterValue _output_get "Color" (Variables|Pointer|GetBeamColor) :!class /Script/Engine.MaterialInstanceDynamic)
      (Rendering|Material|SetScalarParameterValue _output_get "Emissive" (Variables|Pointer|GetBeamEmissive) :!class /Script/Engine.MaterialInstanceDynamic))
    (:then_2
      (bind _returnvalue_4 (Rendering|Material|CreateDynamicMaterialInstance (Variables|Default|GetDotMesh) 0 "/Game/ToolsR1/LaserPointerTool/M_LaserDot.M_LaserDot" "None" :!class /Script/Engine.PrimitiveComponent))
      (bind _output_get_2 (Variables|Pointer|SetDotMaterial _returnvalue_4))
      (Rendering|Material|SetVectorParameterValue _output_get_2 "Color" (Variables|Pointer|GetBeamColor) :!class /Script/Engine.MaterialInstanceDynamic)
      (Rendering|Material|SetScalarParameterValue _output_get_2 "Emissive" (Variables|Pointer|GetBeamEmissive) :!class /Script/Engine.MaterialInstanceDynamic))))

(fn FLaserPointer
  (bind _motioncontroller (Variables|Default|GetMotionController))
  (bind _beammesh (Variables|Default|GetBeamMesh))
  (bind _dotmesh (Variables|Default|GetDotMesh))
  (bind _beamthickness (Variables|Pointer|GetBeamThickness))
  (bind _beamlength (Variables|Pointer|GetBeamLength))
  (bind _returnvalue (Transformation|GetWorldLocation _motioncontroller))
  (bind _returnvalue_2 (* _beamthickness 0.01))
  (bind _outhit (Collision|LineTraceByChannel _returnvalue (+ (* (Math|Vector|GetForwardVector _motioncontroller) (Variables|Pointer|GetTraceDistance)) _returnvalue) "TraceTypeQuery1" false 0 "None" true "(R=0.000000,G=0.500000,B=1.000000,A=1.000000)"))
  (if (.bblockinghit _outhit)
    (Variables|Pointer|SetHitActor (.hitactor _outhit))
    (bind _output_get (Variables|Pointer|SetBeamLengthNew (* (* (/ (- (.distance _outhit) (Variables|Pointer|GetBeamOriginOffset)) _beamlength) _beamlength) 0.01)))
    (Transformation|SetWorldScale3D _beammesh (Math|Vector|MakeVector _returnvalue_2 _returnvalue_2 _output_get))
    (Development|SetHiddeninGame _dotmesh false false)
    (else
      (Variables|Pointer|SetHitActor 0)
      (bind _output_get_2 (Variables|Pointer|SetBeamLengthNew (* (Variables|Pointer|GetBeamLength) 0.01)))
      (Transformation|SetWorldScale3D _beammesh (Math|Vector|MakeVector _returnvalue_2 _returnvalue_2 _output_get_2))
      (Development|SetHiddeninGame _dotmesh true false)))
  (Transformation|SetRelativeLocation _beammesh (Math|Vector|MakeVector (Math|Float|Absolute(Float) (+ (* (Variables|Pointer|GetBeamLengthNew) 0.5 1e+02) (Variables|Pointer|GetBeamOriginOffset))) 0.0 0.0) false false)
  (Rendering|Material|SetScalarParameterValue (Variables|Pointer|GetBeamMaterial) "GradientFalloffUVs" (/ (Variables|Pointer|GetBeamLengthNew) (* (Variables|Pointer|GetBeamFadeLength) 0.01)) :!class /Script/Engine.MaterialInstanceDynamic)
  (Transformation|SetWorldLocationAndRotation (Variables|Default|GetDotMesh) (.location _outhit) (Math|Rotator|MakeRotator (.Roll (Math|Rotator|BreakRotator (Math|Conversions|RotationFromXVector (.normal _outhit)))) (+ (.Pitch (Math|Rotator|BreakRotator (Math|Conversions|RotationFromXVector (.normal _outhit)))) 9e+01) (.Yaw (Math|Rotator|BreakRotator (Math|Conversions|RotationFromXVector (.normal _outhit))))) false false))

(fn FSoftLock
  (params (Component_Scene :type Scene%20Component%20Object%20Reference))
  (bind _returnvalue (Game|GetPlayerCameraManager 0))
  (bind _returnvalue_2 (Camera|GetCameraLocation _returnvalue))
  (bind _output_get (Variables|Default|SetLocationTarget (+ _returnvalue_2 (* (Transformation|GetActorForwardVector _returnvalue) (Variables|Default|GetWidgetDistance)))))
  (bind _output_get_2 (Variables|Default|SetLocationCurrent (Math|Vector|Lerp(Vector) (Variables|Default|GetLocationCurrent) _output_get (* (Utilities|Time|GetWorldDeltaSeconds) (Variables|Default|GetWidgetInterpSpeed)))))
  (Transformation|SetWorldLocation Component_Scene _output_get_2 false false)
  (Transformation|SetWorldRotation Component_Scene (Math|Rotator|FindLookatRotation (Transformation|GetWorldLocation Component_Scene) _returnvalue_2) false false))

(fn FDrawRayTraceControllertoCollision
  (bind _motioncontroller (Variables|Default|GetMotionController))
  (bind _tracemeshbeam (Variables|Default|GetTraceMeshBeam))
  (bind _beamthickness_0 (Variables|Trace|GetBeamThickness_0))
  (bind _beamlength_0 (Variables|Trace|GetBeamLength_0))
  (bind _tracemeshend (Variables|Default|GetTraceMeshEnd))
  (bind _returnvalue (Transformation|GetWorldLocation _motioncontroller))
  (bind _returnvalue_2 (* _beamthickness_0 0.01))
  (bind _outhit (Collision|LineTraceByChannel _returnvalue (+ (* (Math|Vector|GetForwardVector _motioncontroller) (Variables|Trace|GetTraceDistance_0)) _returnvalue) "TraceTypeQuery1" false 0 "None" true "(R=0.000000,G=0.500000,B=1.000000,A=1.000000)"))
  (if (.bblockinghit _outhit)
    (Variables|Trace|SetHitActor_0 (.hitactor _outhit))
    (bind _output_get (Variables|Trace|SetBeamLengthNew_0 (* (* (/ (- (.distance _outhit) (Variables|Trace|GetBeamOriginOffset_0)) _beamlength_0) _beamlength_0) 0.01)))
    (Transformation|SetWorldScale3D _tracemeshbeam (Math|Vector|MakeVector _returnvalue_2 _returnvalue_2 _output_get))
    (Development|SetHiddeninGame _tracemeshend false false)
    (else
      (Variables|Trace|SetHitActor_0 0)
      (bind _output_get_2 (Variables|Trace|SetBeamLengthNew_0 (* (Variables|Trace|GetBeamLength_0) 0.01)))
      (Transformation|SetWorldScale3D _tracemeshbeam (Math|Vector|MakeVector _returnvalue_2 _returnvalue_2 _output_get_2))
      (Development|SetHiddeninGame _tracemeshend false false)))
  (Transformation|SetRelativeLocation _tracemeshbeam (Math|Vector|MakeVector (Math|Float|Absolute(Float) (+ (* (Variables|Trace|GetBeamLengthNew_0) 0.5 1e+02) (Variables|Trace|GetBeamOriginOffset_0))) 0.0 0.0) false false)
  (Transformation|SetWorldLocationAndRotation (Variables|Default|GetTraceMeshEnd) (.location _outhit) (Math|Rotator|MakeRotator (.Roll (Math|Rotator|BreakRotator (Math|Conversions|RotationFromXVector (.normal _outhit)))) (+ (.Pitch (Math|Rotator|BreakRotator (Math|Conversions|RotationFromXVector (.normal _outhit)))) 9e+01) (.Yaw (Math|Rotator|BreakRotator (Math|Conversions|RotationFromXVector (.normal _outhit))))) false false))

(fn FConstructTraceBeam
  (bind _beamthickness_0 (Variables|Trace|GetBeamThickness_0))
  (bind _beamlength_0 (Variables|Trace|GetBeamLength_0))
  (bind _tracemeshbeam (Variables|Default|GetTraceMeshBeam))
  (bind _returnvalue (* _beamthickness_0 0.01))
  (Utilities|FlowControl|Sequence
    (:then_0
      (Transformation|SetWorldScale3D _tracemeshbeam (Math|Vector|MakeVector _returnvalue _returnvalue (* _beamlength_0 0.01)))
      (Transformation|SetRelativeLocation _tracemeshbeam (Math|Vector|MakeVector (Math|Float|Absolute(Float) (+ (* _beamlength_0 0.5) (* (Variables|Trace|GetBeamOriginOffset_0) 1.0))) 0.0 0.0) false false)
      (Transformation|SetWorldScale3D (Variables|Default|GetTraceMeshEnd) (Math|Conversions|ToVector(Float) (Variables|Trace|GetDotSize_0))))
    (:then_1
      (bind _returnvalue_2 (Rendering|Material|CreateDynamicMaterialInstance (Variables|Default|GetTraceMeshBeam) 0 "/Game/Materials/M_Solid_Color.M_Solid_Color" "None" :!class /Script/Engine.PrimitiveComponent))
      (bind _output_get (Variables|Trace|SetBeamMaterial_0 _returnvalue_2))
      (Rendering|Material|SetVectorParameterValue _output_get "Color" (Variables|Trace|GetBeamColor_0) :!class /Script/Engine.MaterialInstanceDynamic))
    (:then_2
      (bind _returnvalue_3 (Rendering|Material|CreateDynamicMaterialInstance (Variables|Default|GetTraceMeshEnd) 0 "/Game/Materials/M_Solid_Color.M_Solid_Color" "None" :!class /Script/Engine.PrimitiveComponent))
      (bind _output_get_2 (Variables|Trace|SetDotMaterial_0 _returnvalue_3))
      (Rendering|Material|SetVectorParameterValue _output_get_2 "Color" (Variables|Trace|GetHitColor_0) :!class /Script/Engine.MaterialInstanceDynamic))))

(fn FShrinkBeam
  (Transformation|SetWorldScale3D (Variables|Default|GetTraceMeshBeam) "0, 0, 0")
  (Transformation|SetWorldScale3D (Variables|Default|GetTraceMeshEnd) "0, 0, 0"))