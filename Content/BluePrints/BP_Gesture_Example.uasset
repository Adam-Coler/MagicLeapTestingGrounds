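; Example Blueprint that displays each hand's detected gesture and its confidence percentage on left and right text elements.
; A looping timer refreshes both hands at a configurable rate, while a gesture-detected event updates the affected hand as soon as a new gesture arrives.
; Both paths feed SetHandText, which maps the gesture to a label and formats the confidence, showing a fixed 100% when no hand is present.
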(event Custom|DetectedNewGesture
  (params (Gesture :type EHandTrackingGesture%20Enum :default "Finger") (Hand :type E_HandType%20Enum :default "NewEnumerator0"))
  ;[1 0.6771 0.6771] Change text to match new gesture
  (CallFunction|SetHandText Hand Gesture))

(event EventBeginPlay
  ;[0.165 1 0.1379] Initialize
  (Utilities|FlowControl|Sequence
    (:then_0
      (Utilities|Time|SetTimerbyFunctionName self "RefreshGestureText" (Variables|Default|GetConfidenceTextUpdateRate) true))
    (:then_1
      (EventDispatchers|BindEventtoOnGestureDetected (delegate Custom|DetectedNewGesture)))))

(fn ConstructionScript
  (|CallParentFunction))

(fn SetHandText
  (params (HandF :type E_HandType%20Enum :default "NewEnumerator0") (CurrentGestureF :type EHandTrackingGesture%20Enum :default "Finger"))
  (bind _returnvalue (Utilities|Enum|Equal(Enum) HandF "NewEnumerator0"))
  (bind _confidence (Class|MagicLeapHandTrackingFunctionLibrary|GetCurrentGestureConfidence (select _returnvalue "Left" "Right")))
  (Rendering|Components|TextRender|SetText (select _returnvalue (Variables|Default|GetText%20-%20Left%20Gesture) (Variables|Default|GetText%20-%20Right%20Gesture)) (Utilities|Text|ToText(String) (Utilities|String|Append (select _returnvalue "Left: " "Right: ") (Utilities|Select :Index CurrentGestureF :Finger "Finger" :Fist "Fist" :Pinch "Pinch" :Thumb "Thumb" :L "L" :OpenHandBack "OpenHandBack" :Ok "Ok" :C "C" :NoPose "" :NoHand "NoHand") ", " (select (Utilities|Enum|Equal(Enum) CurrentGestureF "NoHand") "100" (Utilities|String|ToString(Text) (Utilities|Text|ToText(Float) (* _confidence 1e+02) "HalfToEven" false true 1 324 0 2))) "% confidence"))))

(fn RefreshGestureText
  (Utilities|FlowControl|Sequence
    (:then_0
      (CallFunction|SetHandText "NewEnumerator0" (CallFunction|GetCurrentGesture "NewEnumerator0")))
    (:then_1
      (CallFunction|SetHandText "NewEnumerator1" (CallFunction|GetCurrentGesture "NewEnumerator1")))))